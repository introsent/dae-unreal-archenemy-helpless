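; Base projectile that deals damage to whatever its Collision component hits or overlaps, then destroys itself.
; Both collision events feed ProcessCollision, which skips invalid actors and those carrying IgnoreTag, leaving the projectile alive.
; Damage goes through the BPI_Damagable interface to the struck actor and to each of its implementing components, stopping the component loop if the actor becomes invalid.
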(event OnComponentHit(Collision)
  (params (HitComponent :type Primitive%20Component%20Object%20Reference) (OtherActor :type Actor%20Object%20Reference) (OtherComp :type Primitive%20Component%20Object%20Reference) (NormalImpulse :type Vector :default "0, 0, 0") (Hit :type Hit%20Result%20Structure%20%28by%20ref%29))
  (CallFunction|ProcessCollision OtherActor))

(event OnComponentBeginOverlap(Collision)
  (params (OverlappedComponent :type Primitive%20Component%20Object%20Reference) (OtherActor :type Actor%20Object%20Reference) (OtherComp :type Primitive%20Component%20Object%20Reference) (OtherBodyIndex :type Integer) (bFromSweep :type Boolean) (SweepResult :type Hit%20Result%20Structure%20%28by%20ref%29))
  (CallFunction|ProcessCollision OtherActor))

(event EventBeginPlay)

(event Collision|EventActorBeginOverlap
  (params (OtherActor :type Actor%20Object%20Reference)))

(event EventTick
  (params (DeltaSeconds :type Float%20%28single-precision%29)))

(fn ConstructionScript)

(fn ProcessCollision
  (params (otherActor :type Actor%20Object%20Reference))
  (bind _returnvalue (Class|Actor|GetComponentsbyInterface otherActor "/Game/Blueprints/BPI_Damagable.BPI_Damagable_C"))
  ;[1 1 1] Check if hit an actor
  (Utilities|IsValid otherActor
    (:Is%20Valid
      (if (not (Actor|ActorHasTag otherActor (Variables|Default|GetignoreTag)))
        (Utilities|FlowControl|Sequence
          (:then_0
            ;[1 1 1] BPI_Damagable on hit actor
            (if (Utilities|DoesObjectImplementInterface otherActor "/Game/Blueprints/BPI_Damagable.BPI_Damagable_C")
              (Class|BPIDamagable|DoDamage(Message) otherActor (Variables|Default|GetdamageAmount))))
          (:then_1
            ;[1 1 1] Get all component that implement BPI_Demagable and do damage
            (Utilities|IsValid otherActor
              (:Is%20Valid
                (bind _index (Utilities|FlowControl|ForLoopwithBreak 0 (- (Utilities|Array|Length _returnvalue) 1) :!label _label)
                  (:LoopBody
                    (Class|BPIDamagable|DoDamage(Message) (Utilities|Array|Get(acopy) _returnvalue _index) (Variables|Default|GetdamageAmount))
                    (Utilities|IsValid otherActor
                      (:Is%20Not%20Valid
                        (goto _label Break))))))))
          (:then_2
            ;[1 1 1] Destroy
            (Actor|DestroyActor)))))))