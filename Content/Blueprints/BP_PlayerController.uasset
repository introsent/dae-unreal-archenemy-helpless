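; Player controller for a side-view grappling-hook character moving on the XZ plane, also setting up input, HUD and restart.
; Mouse clicks are deprojected onto a fixed-Y plane, turning the character and aiming a fixed-length hook trace that sets GrabPoint.
; On a hit, RMB grapples in Flying mode, suspending movement input, while LMB swings in Falling mode and launches on release.
; BP_Hook's cable visualizes both hits and misses, with attach and detach sounds.
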(event Input|EnhancedActionEvents|EnhancedInputActionIA_RestartInput
  (params (ActionValue :type Boolean) (ElapsedSeconds :type Float%20%28double-precision%29) (TriggeredSeconds :type Float%20%28double-precision%29) (InputAction :type Input%20Action%20Object%20Reference :default "/Game/Input/Actions/IA_RestartInput.IA_RestartInput"))
  (bind _asbp_game_mode (Utilities|Casting|CastToBP_GameMode (Game|GetGameMode)))
  (Default|Restart _asbp_game_mode))

(event Input|EnhancedActionEvents|EnhancedInputActionIA_PlayerInput
  (params (ActionValue :type Vector%202D%20Structure) (ElapsedSeconds :type Float%20%28double-precision%29) (TriggeredSeconds :type Float%20%28double-precision%29) (InputAction :type Input%20Action%20Object%20Reference :default "/Game/Input/Actions/IA_PlayerInput.IA_PlayerInput"))
  (bind _returnvalue (Pawn|GetControlledPawn))
  (bind _returnvalue_2 (Pawn|GetControlledPawn))
  (bind _returnvalue_3 (Class|Pawn|GetLastMovementInputVector _returnvalue_2))
  ;[1 1 1] Handle Movement Input
  (Variables|Default|SetCurrentRightLeftInput (.x ActionValue))
  (if (not (Variables|Default|GetisGrappling))
    (Utilities|IsValid _returnvalue
      (:Is%20Valid
        (Pawn|Input|AddMovementInput _returnvalue (Math|Vector|ClampVectorSize (Math|Vector|MakeVector (.x ActionValue) 0.0 (.y ActionValue)) 0.0 1.0) 1.0 false)
        (Utilities|IsValid _returnvalue_2
          (:Is%20Valid
            (if (> (Math|Vector|VectorLengthSquared _returnvalue_3) 0.0)
              (Pawn|SetControlRotation (Math|Rotator|MakeRotator 0.0 0.0 (.yaw (Math|Conversions|RotationFromXVector _returnvalue_3)))))))))))

(event EventBeginPlay
  (bind _returnvalue (PlayerController|LocalPlayerSubsystems|GetEnhancedInputLocalPlayerSubsystem))
  (Utilities|FlowControl|Sequence
    (:then_0
      ;[1 1 1] Enable default input mapping context
      (Variables|Default|SetbShowMouseCursor true)
      (Utilities|IsValid _returnvalue
        (:Is%20Valid
          (Input|AddMappingContext _returnvalue "/Game/Input/IMC_Default.IMC_Default" 0 "(bIgnoreAllPressedKeysUntilRelease=True,bForceImmediately=False,bNotifyUserSettings=False)"))))
    (:then_1
      ;[1 1 1] Setup HUD
      (bind _returnvalue_2 (UserInterface|CreateWidget "/Game/Blueprints/BPW_GameHUD.BPW_GameHUD_C" self))
      (UserInterface|Viewport|AddtoViewport _returnvalue_2 0))))

(event Input|ActionEvents|InputActionRMB_Action
  (params (Key :type Key%20Structure :default "None"))
  (bind (_diddeproject _clickprojectionlocation) (CallFunction|DeprojectScreenLocationtoWorld))
  (bind _playercharacter (CallFunction|GetPlayerCharacterReference))
  (bind _playercharacter_2 (CallFunction|GetPlayerCharacterReference))
  (bind (_start _end) (CallFunction|GetStartandEndLocationforHookTrace _clickprojectionlocation))
  (bind _charactermovement (Variables|/Script/Engine.Character|GetCharacterMovement _playercharacter_2))
  (bind _charactermovement_2 (Variables|/Script/Engine.Character|GetCharacterMovement _playercharacter))
  ;[1 0.5664 0.7406] On RMB grab to the position of the click projected to 2D and rotate character toward the position for grappling mechanic
  (:Pressed
    (if _diddeproject
      (Utilities|FlowControl|Sequence
        (:then_0
          (bind (_outhit _returnvalue) (Collision|LineTraceByChannel _start _end "TraceTypeQuery1" true (Utilities|Array|MakeArray (Pawn|GetControlledPawn)) "None" :!label _label))
          (if _returnvalue
            (Variables|Default|SetgrabPoint (.location _outhit))
            (Variables|Default|SetisSwinging false)
            (Variables|Default|SetisGrappling true)
            ;;[1 1 1] When pressing set movement mode to Flying
            (Utilities|IsValid _playercharacter_2
              (:Is%20Valid
                (Utilities|IsValid _charactermovement
                  (:Is%20Valid
                    (Pawn|Components|CharacterMovement|SetMovementMode _charactermovement "MOVE_Flying" 0)
                    (bind _returnvalue_2 (Actor|GetActorOfClass "/Game/Blueprints/BP_Hook.BP_Hook_C"))
                    (Utilities|IsValid _returnvalue_2
                      (:Is%20Valid
                        ;;[1 1 1] When pressed make hook visible and attach sound
                        (Audio|SpawnSoundAttached "/Game/Audio/hook_attached.hook_attached" (Variables|/Game/Blueprints/BP_Hook.BP_Hook_C|GetCable _returnvalue_2) "None" "0, 0, 0" "0, 0, 0" "KeepRelativeOffset" false 1.0 1.0 0.0 0 0)
                        (Rendering|SetVisibility (Variables|/Game/Blueprints/BP_Hook.BP_Hook_C|GetCable _returnvalue_2) true false)))))))
            (else
              ;;[1 1 1] Visualize hook even when not connected
              (Variables|Default|SetgrabPoint (.traceend _outhit))
              (Variables|Default|SetisSwinging false)
              (Variables|Default|SetisGrappling false)
              (bind _returnvalue_3 (Actor|GetActorOfClass "/Game/Blueprints/BP_Hook.BP_Hook_C"))
              (Utilities|IsValid _returnvalue_3
                (:Is%20Valid
                  (Rendering|SetVisibility (Variables|/Game/Blueprints/BP_Hook.BP_Hook_C|GetCable _returnvalue_3) true false))))))
        (:then_1
          (CallFunction|SetControlledCharacterRotation _clickprojectionlocation))
        (:then_2
          (if (not (Variables|Default|GetisGrappling))
            (goto _label))))))
  (:Released
    (Variables|Default|SetisGrappling false)
    ;;[1 1 1] When released set movement mode to Falling
    (Utilities|IsValid _playercharacter
      (:Is%20Valid
        (Utilities|IsValid _charactermovement_2
          (:Is%20Valid
            (Pawn|Components|CharacterMovement|SetMovementMode _charactermovement_2 "MOVE_Falling" 0)
            ;;[1 1 1] When released make hook invisible
            (bind _returnvalue_4 (Actor|GetActorOfClass "/Game/Blueprints/BP_Hook.BP_Hook_C"))
            (Utilities|IsValid _returnvalue_4
              (:Is%20Valid
                (Rendering|SetVisibility (Variables|/Game/Blueprints/BP_Hook.BP_Hook_C|GetCable _returnvalue_4) false false)
                (Audio|SpawnSoundAttached "/Game/Audio/hook_deattached.hook_deattached" (Variables|/Game/Blueprints/BP_Hook.BP_Hook_C|GetCable _returnvalue_4) "None" "0, 0, 0" "0, 0, 0" "KeepRelativeOffset" false 1.0 1.0 0.0 0 0)))))))))

(event Input|ActionEvents|InputActionLMB_Action
  (params (Key :type Key%20Structure :default "None"))
  (bind (_diddeproject _clickprojectionlocation) (CallFunction|DeprojectScreenLocationtoWorld))
  (bind _playercharacter (CallFunction|GetPlayerCharacterReference))
  (bind _playercharacter_2 (CallFunction|GetPlayerCharacterReference))
  (bind (_start _end) (CallFunction|GetStartandEndLocationforHookTrace _clickprojectionlocation))
  (bind _charactermovement (Variables|/Script/Engine.Character|GetCharacterMovement _playercharacter))
  (bind _charactermovement_2 (Variables|/Script/Engine.Character|GetCharacterMovement _playercharacter_2))
  ;[1 0.5664 0.7406] On LMB grab to the position of the click projected to 2D and rotate character toward the position for swinging mechanic
  (:Pressed
    (if _diddeproject
      (Utilities|FlowControl|Sequence
        (:then_0
          (bind (_outhit _returnvalue) (Collision|LineTraceByChannel _start _end "TraceTypeQuery1" true (Utilities|Array|MakeArray (Pawn|GetControlledPawn)) "None" :!label _label))
          (if _returnvalue
            (Variables|Default|SetgrabPoint (.location _outhit))
            (Variables|Default|SetisGrappling false)
            (Variables|Default|SetisSwinging true)
            ;;[1 1 1] When pressing set movement mode to Flying
            (Utilities|IsValid _playercharacter
              (:Is%20Valid
                (Utilities|IsValid _charactermovement
                  (:Is%20Valid
                    (Pawn|Components|CharacterMovement|SetMovementMode _charactermovement "MOVE_Falling" 0)
                    (bind _returnvalue_2 (Actor|GetActorOfClass "/Game/Blueprints/BP_Hook.BP_Hook_C"))
                    (Utilities|IsValid _returnvalue_2
                      (:Is%20Valid
                        ;;[1 1 1] When pressed make hook visible and attach sound
                        (Audio|SpawnSoundAttached "/Game/Audio/hook_attached.hook_attached" (Variables|/Game/Blueprints/BP_Hook.BP_Hook_C|GetCable _returnvalue_2) "None" "0, 0, 0" "0, 0, 0" "KeepRelativeOffset" false 1.0 1.0 0.0 0 0)
                        (Rendering|SetVisibility (Variables|/Game/Blueprints/BP_Hook.BP_Hook_C|GetCable _returnvalue_2) true false)))))))
            (else
              ;;[1 1 1] To visualize hook even when not connected
              (Variables|Default|SetgrabPoint (.traceend _outhit))
              (Variables|Default|SetisSwinging false)
              (Variables|Default|SetisGrappling false)
              (bind _returnvalue_3 (Actor|GetActorOfClass "/Game/Blueprints/BP_Hook.BP_Hook_C"))
              (Utilities|IsValid _returnvalue_3
                (:Is%20Valid
                  (Rendering|SetVisibility (Variables|/Game/Blueprints/BP_Hook.BP_Hook_C|GetCable _returnvalue_3) true false))))))
        (:then_1
          (CallFunction|SetControlledCharacterRotation _clickprojectionlocation))
        (:then_2
          (if (not (Variables|Default|GetisSwinging))
            (goto _label))))))
  (:Released
    ;;[1 1 1] Release input logic
    (if (Variables|Default|GetisSwinging)
      (Variables|Default|SetisSwinging false)
      ;;;[1 1 1] When released set movement mode to Falling
      (Utilities|IsValid _playercharacter_2
        (:Is%20Valid
          (Default|LaunchwithForce _playercharacter_2)
          (Utilities|IsValid _charactermovement_2
            (:Is%20Valid
              (Pawn|Components|CharacterMovement|SetMovementMode _charactermovement_2 "MOVE_Falling" 0)
              ;;;[1 1 1] When released make hook invisible
              (bind _returnvalue_4 (Actor|GetActorOfClass "/Game/Blueprints/BP_Hook.BP_Hook_C"))
              (Rendering|SetVisibility (Variables|/Game/Blueprints/BP_Hook.BP_Hook_C|GetCable _returnvalue_4) false false)
              (Audio|SpawnSoundAttached "/Game/Audio/hook_deattached.hook_deattached" (Variables|/Game/Blueprints/BP_Hook.BP_Hook_C|GetCable _returnvalue_4) "None" "0, 0, 0" "0, 0, 0" "KeepRelativeOffset" false 1.0 1.0 0.0 0 0))))))))

(fn ConstructionScript)

(fn GetPlayerCharacterReference
  (bind _asbp_player_character (Utilities|Casting|CastToBP_PlayerCharacter (Pawn|GetControlledPawn)))
  (return _asbp_player_character))

(fn SetControlledCharacterRotation
  (params (MouseHitLocation :type Vector))
  (bind (_x _y _z) (Math|Vector|BreakVector MouseHitLocation))
  (bind _returnvalue (Pawn|GetControlledPawn))
  (bind _returnvalue_2 (Transformation|GetActorLocation _returnvalue))
  (bind (_x_2 _y_2 _z_2) (Math|Vector|BreakVector _returnvalue_2))
  ;[1 1 1] Set the controller rotation
  (Pawn|SetControlRotation (Math|Rotator|MakeRotator 0.0 0.0 (.yaw (Math|Rotator|FindLookatRotation (Math|Vector|MakeVector _x_2 0.0 _z_2) (Math|Vector|MakeVector _x 0.0 _z))))))

(fn GetStartandEndLocationforHookTrace
  (params (MouseHitLocation :type Vector))
  (bind _returnvalue (Pawn|GetControlledPawn))
  (bind _returnvalue_2 (Transformation|GetActorLocation _returnvalue))
  (bind _returnvalue_3 (- MouseHitLocation _returnvalue_2))
  (bind _returnvalue_4 (Math|Vector|Normalize _returnvalue_3))
  ;[1 1 1] Calculate start and end location for line trace of Hook
  (return _returnvalue_2 (+ _returnvalue_2 (* (Math|Vector|Normalize (Math|Vector|MakeVector (.x _returnvalue_4) 0.0 (.z _returnvalue_4))) 1e+03))))

(fn DeprojectScreenLocationtoWorld
  (bind (_locationx _locationy) (Game|Player|GetMousePosition))
  (bind _self self)
  (bind _returnvalue (Math|Vector2D|MakeVector2D _locationx _locationy))
  (bind (_worldposition _worlddirection _returnvalue_2) (Class|GameplayStatics|DeprojectScreentoWorld _self _returnvalue))
  (return _returnvalue_2 (+ _worldposition (* _worlddirection (/ (- 4e+02 (.Y (Math|Vector|BreakVector _worldposition))) (.Y (Math|Vector|BreakVector _worlddirection)))))))