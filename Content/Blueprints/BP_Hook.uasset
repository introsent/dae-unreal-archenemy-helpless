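; BP_Hook is a hook actor with a cable and a physics constraint, set up for a player swing mechanic that is not wired up.
; On BeginPlay it spawns a BP_CableEndpoint, attaches the cable's end to it and deactivates the constraint.
; Disconnected logic would constrain the player mesh to the endpoint with distance-based limits, but ActivateSwing and DeactivateSwing are empty.
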(event Custom|ActivateSwing
  ;[1 1 1] Swing activation logic
)

(event Custom|DeactivateSwing
  ;[1 1 1] Deactivate swing
)

(event EventBeginPlay
  ;[1 1 1] Spawn EndPoint actor and Attach end of the Hook to it
  (Game|SpawnActorfromClass "/Game/Blueprints/BP_CableEndpoint.BP_CableEndpoint_C" (Transformation|GetWorldTransform (Variables|Default|GetCable)) "Undefined" "MultiplyWithRoot" 0 0)
  (bind _returnvalue (Actor|GetActorOfClass "/Game/Blueprints/BP_CableEndpoint.BP_CableEndpoint_C"))
  (Class|CableComponent|SetAttachEndto (Variables|Default|GetCable) _returnvalue "None" "None")
  (Components|Activation|SetActive (Variables|Default|GetSwingPhysicsConstraint) false false))

(event Collision|EventActorBeginOverlap
  (params (OtherActor :type Actor%20Object%20Reference)))

(event EventTick
  (params (DeltaSeconds :type Float%20%28single-precision%29)))

(fn ConstructionScript)