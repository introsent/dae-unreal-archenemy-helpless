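; Enemy character that patrols between two points with a visible vision cone and shoots the player on sight.
; A fan of line traces from the head in the XZ plane builds a triangulated dynamic mesh, redrawn only when hits change.
; When more than five rays hit the player, it rotates the weapon socket toward a random hit point and fires once until detection drops.
; BeginPlay spawns the weapon, and construction previews the cone and tints the body.
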(event Custom|MovePatrol
  ;[1 1 1] Patrol
  (AI|AIMoveTo self (Utilities|Array|Get(acopy) (Variables|Default|GetpatrolLocation) (Variables|Default|Getlocations)) 0 5.0 false
    (:OnSuccess
      (Utilities|FlowControl|Delay 0.5)
      (CallFunction|MovePatrol)
      (Math|Integer|IncrementInt (Variables|Default|Getlocations)
        (:%20%20
          (if (== (Variables|Default|Getlocations) 2)
            (Variables|Default|Setlocations 0)))))))

(event EventBeginPlay
  (bind _startweapon (Variables|Default|GetstartWeapon))
  (|CallParentFunction)
  (Transformation|AttachComponentToComponent (Variables|Default|GetWeaponSocket) (Variables|Character|GetMesh) "WeaponSocket" "KeepRelative" "KeepRelative" "KeepRelative" true)
  ;[1 1 1] Store and attach the weapon
  (bind _asbp_base_weapon (Utilities|Casting|CastToBP_BaseWeaponClass (Class|KismetMathLibrary|SelectClass _startweapon "/Game/Blueprints/BP_BaseWeapon.BP_BaseWeapon_C" (Utilities|IsValidClass _startweapon))))
  (bind _returnvalue (Game|SpawnActorfromClass _asbp_base_weapon (Transformation|GetWorldTransform (Variables|Default|GetGunSocket)) "Undefined" "MultiplyWithRoot" 0 0))
  (bind _output_get (Variables|Default|SetcurrentWeapon _returnvalue))
  (Transformation|AttachComponentToComponent _output_get (Variables|Default|GetWeaponSocket) "" "SnapToTarget" "SnapToTarget" "SnapToTarget" true)
  (bind _hitresult (CallFunction|TraceLines))
  (Variables|Default|SetlastHitResult _hitresult)
  (CallFunction|MovePatrol))

(event Collision|EventActorBeginOverlap
  (params (OtherActor :type Actor%20Object%20Reference)))

(event EventTick
  (params (DeltaSeconds :type Float%20%28single-precision%29))
  (bind _weaponsocket (Variables|Default|GetWeaponSocket))
  (|CallParentFunction DeltaSeconds)
  ;[1 1 1] Trace line and update polygon only when output hits array has changed
  (bind _hitresult (CallFunction|TraceLines))
  (Variables|Default|SetcurrentHitResult _hitresult)
  (if (not (Utilities|Array|Identical (Variables|Default|GetlastHitResult) (Variables|Default|GetcurrentHitResult)))
    (DynamicMesh|Reset (Variables|Default|GetdynamicDetectionMesh))
    (Class|GeometryScriptLibraryMeshPrimitiveFunctions|AppendTriangulatedPolygon :TargetMesh (Variables|Default|GetdynamicDetectionMesh) :PolygonVertices (CallFunction|HitResultto2DVertices (Variables|Default|GetcurrentHitResult)) :Debug 0)
    ;;[0.8401 0.3175 1] Make sure bullet will fire once when hit the player
    (bind (_tofire _position) (CallFunction|FireifHitwithPlayer (Variables|Default|GetcurrentHitResult)))
    (if _tofire
      (if (not (Variables|Default|GethasFired))
        ;;;[1 1 1] Check forward vector of weapon socket
        (if (> (.y (Math|Vector|GetForwardVector (Variables|Default|GetWeaponSocket))) 0.0)
          (Transformation|SetWorldRotation _weaponsocket (Class|KismetMathLibrary|NegateRotator (Math|Rotator|MakeRotator (.Roll (Math|Rotator|BreakRotator (Math|Rotator|FindLookatRotation (Transformation|GetWorldLocation _weaponsocket) _position))) (.Pitch (Math|Rotator|BreakRotator (Math|Rotator|FindLookatRotation (Transformation|GetWorldLocation _weaponsocket) _position))) -9e+01)) false false)
          (else
            (Transformation|SetWorldRotation (Variables|Default|GetWeaponSocket) (Class|KismetMathLibrary|NegateRotator (Math|Rotator|MakeRotator (.Roll (Math|Rotator|BreakRotator (Class|KismetMathLibrary|NegateRotator (Math|Rotator|FindLookatRotation (Transformation|GetWorldLocation _weaponsocket) _position)))) (.Pitch (Math|Rotator|BreakRotator (Class|KismetMathLibrary|NegateRotator (Math|Rotator|FindLookatRotation (Transformation|GetWorldLocation _weaponsocket) _position)))) 9e+01)) false false)))
        (CallFunction|Fire _position)
        (Variables|Default|SethasFired true)
        (Variables|Default|SetlastHitResult (Variables|Default|GetcurrentHitResult) :!label _label))
      (else
        (Transformation|SetRelativeRotation (Variables|Default|GetWeaponSocket) "0, 0, 0" true false)
        (Variables|Default|SethasFired false)
        (goto _label)))))

(fn ConstructionScript
  (Utilities|FlowControl|Sequence
    (:then_0
      ;[1 1 1] Generate dynamic detection mesh and store it
      (bind _returnvalue (AddComponent|AddDynamicMeshComponent false (Math|Transform|MakeTransform "0, 0, 0" "0.000000,0.000000,-90.000000")))
      (bind _output_get (Variables|Default|SetdynamicMeshComponent _returnvalue))
      (bind _returnvalue_2 (DynamicMeshComponent|GetDynamicMesh _output_get))
      (Variables|Default|SetdynamicDetectionMesh _returnvalue_2))
    (:then_1
      ;[1 1 1] Perform linetracing and create and draw polygon
      (bind _hitresult (CallFunction|TraceLines))
      (Class|GeometryScriptLibraryMeshPrimitiveFunctions|AppendTriangulatedPolygon :TargetMesh (Variables|Default|GetdynamicDetectionMesh) :PolygonVertices (CallFunction|HitResultto2DVertices _hitresult) :Debug 0)
      (Rendering|Material|SetMaterial (Variables|Default|GetdynamicMeshComponent) 0 "/Game/Materials/MAT_VisionCone.MAT_VisionCone"))
    (:then_2
      ;[1 1 1] Generate BodyColor
      (bind _returnvalue_3 (Rendering|Material|CreateDynamicMaterialInstance (Variables|Character|GetMesh) 0 0 "None" :!class /Script/Engine.PrimitiveComponent))
      (bind _output_get_2 (Variables|Enemy|SetbodyMaterialInstance _returnvalue_3))
      (Rendering|Material|SetVectorParameterValue _output_get_2 "BodyColor" (Variables|Enemy|GetenemyColor) :!class /Script/Engine.MaterialInstanceDynamic))))

(fn Patrol)

(fn TraceLines
  (bind _mesh (Variables|Character|GetMesh))
  (bind _returnvalue (Transformation|GetSocketLocation _mesh "head"))
  ;[1 1 1] For each vision arc trace a line and write the result to the output array
  (for _index (range 0 (Math|Float|Ceil (/ (Variables|Default|GetvisionArc) (Variables|Default|GettestVisionArc))))
    (bind _outhit (Collision|LineTraceByChannel _returnvalue (+ _returnvalue (Math|Vector|RotateVectorAroundAxis (* (Transformation|GetActorForwardVector) (Variables|Default|GetvisionLength)) (- (Math|Float|Clamp(Float) (* _index (Variables|Default|GettestVisionArc)) (* _index (Variables|Default|GettestVisionArc)) (Variables|Default|GetvisionArc)) (/ (Variables|Default|GetvisionArc) 2.0)) "0.000000,1.000000,0.000000")) "TraceTypeQuery1" false 0 "None"))
    (Utilities|Array|Add (LocalVariables|GetlocalHitResult) _outhit))
  (return (LocalVariables|GetlocalHitResult)))

(fn HitResultto2DVertices
  (params (hitResults :type Array%20of%20Hit%20Result%20Structures))
  ;[1 1 1] Convert output hit results array to an array of 2D vertices in local space
  (Utilities|Array|Add (LocalVariables|Getlocal2DVector) "(X=0.000000,Y=80.000000)")
  (for _array_element hitResults
    (Utilities|Array|Add (LocalVariables|Getlocal2DVector) (Math|Vector2D|MakeVector2D (.X (Math|Vector|BreakVector (Math|Transform|InverseTransformLocation (Transformation|GetActorTransform) (Math|Vector|SelectVector (.location _array_element) (.traceend _array_element) (.bblockinghit _array_element))))) (.Z (Math|Vector|BreakVector (Math|Transform|InverseTransformLocation (Transformation|GetActorTransform) (Math|Vector|SelectVector (.location _array_element) (.traceend _array_element) (.bblockinghit _array_element))))))))
  (return (LocalVariables|Getlocal2DVector)))

(fn FireifHitwithPlayer
  (params (hitResults :type Array%20of%20Hit%20Result%20Structures))
  ;[1 1 1] Additional check to make sure array is empty
  (Utilities|Array|Clear (LocalVariables|GetarrayOfLocations))
  (for _array_element hitResults
    ;[1 1 1] If line hits PlayerCHaracter add hit location to an array
    (Utilities|Casting|CastToBP_PlayerCharacter (.hitactor _array_element))
    (Utilities|Array|Add (LocalVariables|GetarrayOfLocations) (.location _array_element)))
  (if (> (Utilities|Array|Length (LocalVariables|GetarrayOfLocations)) 5)
    (return true (.OutItem (Utilities|Array|Random (LocalVariables|GetarrayOfLocations))))
    (else
      (return false "0, 0, 0"))))

(fn Fire
  (params (positionToShoot :type Vector))
  (bind _currentweapon (Variables|Default|GetcurrentWeapon)
    (:then
      (Default|FirePrimary _currentweapon))
    (:else)))