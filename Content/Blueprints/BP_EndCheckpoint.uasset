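; BP_EndCheckpoint is an end checkpoint actor that adds an explosion effect to the overlap behavior of its parent class.
; On ActorBeginOverlap it calls the parent handler, then spawns the Niagara_Explosion_04 system at its root component's world location.
; The effect fires on every overlap, with no filter on the other actor in this graph.
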(event EventBeginPlay
  (|CallParentFunction) ; This node is disabled and will not be called.\nDrag off pins to build functionality.
)

(event Collision|EventActorBeginOverlap
  (params (OtherActor :type Actor%20Object%20Reference))
  (|CallParentFunction OtherActor)
  (Niagara|SpawnSystematLocation "/Game/MsvFx_Niagara_Explosion_Pack_01/Prefabs/Niagara_Explosion_04.Niagara_Explosion_04" (Transformation|GetWorldLocation (Variables|Default|GetDefaultSceneRoot self))))

(event EventTick
  (params (DeltaSeconds :type Float%20%28single-precision%29))
  (|CallParentFunction DeltaSeconds) ; This node is disabled and will not be called.\nDrag off pins to build functionality.
)

(fn ConstructionScript
  (|CallParentFunction))