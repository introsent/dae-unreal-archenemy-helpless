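; Side-scrolling player character with a grappling hook, locked to a fixed Y plane.
; Spawns a BP_Hook on its mesh, then each tick reads BP_PlayerController state to pin the cable end at the grab point.
; Grappling pulls toward that point with input bias, swinging applies a velocity-based tether force, and LaunchWithForce boosts release momentum.
; Death or falling below MinHeight requests a GameMode respawn and destroys character and hook.
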(event OnDeath(BPAC_Health)
  (CallFunction|Kill))

(event Custom|Launch%20With%20Force
  ;[1 1 1] Launch character when release from swinging
  (Character|LaunchCharacter (* (Transformation|GetVelocity) 2) false false)
  (Variables|/Script/Engine.CharacterMovementComponent|SetAirControl (Variables|Character|GetCharacterMovement) 0.2))

(event EventBeginPlay
  (|CallParentFunction)
  ;[1 1 1] Spawn and attach weapon
  (bind _returnvalue (Game|SpawnActorfromClass (Variables|Default|GethookClass) (Transformation|GetWorldTransform (Variables|Default|GetHookSocket)) "Undefined" "MultiplyWithRoot" 0 0))
  (bind _asbp_hook (Utilities|Casting|CastToBP_Hook _returnvalue))
  (bind _output_get (Variables|Default|SetCurrentHook _asbp_hook))
  (Transformation|AttachComponentToComponent _output_get (Variables|Character|GetMesh) "HookSocket" "SnapToTarget" "SnapToTarget" "SnapToTarget" true))

(event Collision|EventActorBeginOverlap
  (params (OtherActor :type Actor%20Object%20Reference))
  (|CallParentFunction OtherActor) ; This node is disabled and will not be called.\nDrag off pins to build functionality.
)

(event EventTick
  (params (DeltaSeconds :type Float%20%28single-precision%29))
  (bind _returnvalue (Transformation|GetActorLocation))
  (bind _returnvalue_2 (Transformation|GetActorForwardVector))
  (bind _playercontroller (CallFunction|GetPlayerController))
  (bind _playercontroller_2 (CallFunction|GetPlayerController))
  (bind _playercontroller_3 (CallFunction|GetPlayerController))
  (bind _playercontroller_4 (CallFunction|GetPlayerController))
  (bind _returnvalue_3 (Transformation|GetActorLocation))
  (bind _returnvalue_4 (Transformation|GetActorLocation))
  (bind _currenthook (Variables|Default|GetCurrentHook))
  (bind _zipsound (Variables|Default|GetzipSound))
  (bind _currenthook_2 (Variables|Default|GetCurrentHook))
  (bind _cableendpoint (Variables|/Game/Blueprints/BP_Hook.BP_Hook_C|GetcableEndpoint _currenthook_2))
  (bind _cableendpoint_2 (Variables|/Game/Blueprints/BP_Hook.BP_Hook_C|GetcableEndpoint _currenthook))
  (bind _grabpoint (Variables|/Game/Blueprints/BP_PlayerController.BP_PlayerController_C|GetgrabPoint _playercontroller_4))
  (bind _currentrightleftinput (Variables|/Game/Blueprints/BP_PlayerController.BP_PlayerController_C|GetCurrentRightLeftInput _playercontroller_3))
  (bind _grabpoint_2 (Variables|/Game/Blueprints/BP_PlayerController.BP_PlayerController_C|GetgrabPoint _playercontroller_2))
  (bind _returnvalue_5 (Math|Vector|GetUnitDirection(Vector) _returnvalue_4 _grabpoint_2))
  (bind _returnvalue_6 (- _returnvalue _grabpoint))
  (bind _returnvalue_7 (* _returnvalue_2 _currentrightleftinput))
  (bind _returnvalue_8 (* _returnvalue_7 0.7))
  (bind _returnvalue_9 (+ _returnvalue_5 _returnvalue_8))
  (bind _returnvalue_10 (Math|Vector|Normalize _returnvalue_9))
  (bind _returnvalue_11 (* _returnvalue_10 2e+05))
  (bind (_x _y _z) (Math|Vector|BreakVector _returnvalue_11))
  (if (< (.z (Transformation|GetActorLocation self)) (Variables|Default|GetminHeight))
    ;[1 1 1] Kill character when less then min height
    (CallFunction|Kill)
    (else
      (Transformation|SetActorLocation (Math|Vector|MakeVector (.x _returnvalue_3) 4e+02 (.z _returnvalue_3)) false false)
      ;[1 1 1] Set EndPoint to Hit location
      (Utilities|IsValid _playercontroller
        (:Is%20Valid
          (if (Variables|/Game/Blueprints/BP_PlayerController.BP_PlayerController_C|GetisGrappling _playercontroller)
            (Default|SetMode _currenthook)
            (Utilities|IsValid _currenthook
              (:Is%20Valid
                (Utilities|IsValid _cableendpoint_2
                  (:Is%20Valid
                    (if (Variables|Default|GetisGrabPointSetUp)
                      _
                      (else
                        (bind _returnvalue_12 (Transformation|SetActorLocation _cableendpoint_2 (Variables|/Game/Blueprints/BP_PlayerController.BP_PlayerController_C|GetgrabPoint (CallFunction|GetPlayerController)) false true))
                        (Variables|Default|SetisGrabPointSetUp _returnvalue_12)))
                    (Physics|AddForce (Variables|Character|GetCharacterMovement) (Math|Vector|MakeVector _x 0.0 _z))))))
            (else
              ;[1 1 1] Set EndPoint to Hit Location
              (if (Variables|/Game/Blueprints/BP_PlayerController.BP_PlayerController_C|GetisSwinging (CallFunction|GetPlayerController))
                (Default|SetMode _currenthook_2 1)
                (Utilities|IsValid _currenthook_2
                  (:Is%20Valid
                    (Utilities|IsValid _cableendpoint
                      (:Is%20Valid
                        (if (Variables|Default|GetisGrabPointSetUp)
                          _
                          (else
                            (bind _returnvalue_13 (Transformation|SetActorLocation _cableendpoint (Variables|/Game/Blueprints/BP_PlayerController.BP_PlayerController_C|GetgrabPoint (CallFunction|GetPlayerController)) false true))
                            (Variables|Default|SetisGrabPointSetUp _returnvalue_13)))
                        ;[1 1 1] Apply force and let player swing
                        (Physics|AddForce (Variables|Character|GetCharacterMovement) (* (* (Math|Vector|DotProduct (+ (* (* (Transformation|GetActorForwardVector) (Variables|/Game/Blueprints/BP_PlayerController.BP_PlayerController_C|GetCurrentRightLeftInput (CallFunction|GetPlayerController))) 1e+02) (Transformation|GetVelocity)) _returnvalue_6) (Math|Vector|Normalize _returnvalue_6)) -1e+01))))))
                (else
                  ;[1 1 1] Return capsule height back to normal when not in the air
                  (Variables|Default|SetisGrabPointSetUp false)
                  (Utilities|IsValid _zipsound
                    (:Is%20Valid
                      (Audio|Components|Audio|Stop _zipsound))))))))))))

(fn ConstructionScript
  (|CallParentFunction))

(fn GetPlayerController
  (bind _asbp_player_controller (Utilities|Casting|CastToBP_PlayerController (Pawn|GetController)))
  (return _asbp_player_controller))

(fn Kill
  (bind _asbp_game_mode (Utilities|Casting|CastToBP_GameMode (Game|GetGameMode))
    (:then
      (Default|RespawnPlayer _asbp_game_mode))
    (:CastFailed
      _))
  (Actor|DestroyActor (Variables|Default|GetCurrentHook)))