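; Health component that tracks current health against a maximum, resets it to full on BeginPlay and handles damage.
; DoDamage subtracts a clamped amount, calls OnDeath whenever IsDead is true, and returns whether that hit also lowered health while dead.
; IsDead relies on GetHealthPercentage, which divides the integers before converting to double, so any health below maximum reads as zero and dead.
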(event Custom|ResetHealth
  (Variables|Health|SetcurrentHealth (Variables|Health|GetmaxHealth)))

(event EventBeginPlay
  (CallFunction|ResetHealth))

(event EventTick
  (params (DeltaSeconds :type Float%20%28single-precision%29)))

(fn GetHealthPercentage
  (return (Math|Conversions|ToFloat(Integer) (/ (Variables|Health|GetcurrentHealth) (Variables|Health|GetmaxHealth)))))

(fn IsDead
  (return (<= (CallFunction|GetHealthPercentage) 0.0)))

(fn DoDamage
  (params (amount :type Integer))
  (bind _isdead (CallFunction|IsDead))
  (LocalVariables|SetoriginalHealth (Variables|Health|GetcurrentHealth))
  ;[1 1 1] Store adjusted health value
  (bind _output_get (Variables|Health|SetcurrentHealth (Math|Integer|Clamp(Integer) (- (Variables|Health|GetcurrentHealth) amount) 0 (Variables|Health|GetmaxHealth))))
  ;[1 1 1] Did DoDamage cause health to change and drop below 0
  (if _isdead
    (Default|CallOnDeath))
  (return (and _isdead (> (LocalVariables|GetoriginalHealth) _output_get))))